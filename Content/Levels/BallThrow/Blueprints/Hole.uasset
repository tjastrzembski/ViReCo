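; Hole actor for the BallThrow level that judges whether a thrown Ball counts as a hit.
; On actor overlap with a Ball, it fails the try only if the ball touches the Box but not the Capsule; every other case is a hit.
; It prints the result and broadcasts it as a boolean through the VerifyTry dispatcher.
; End overlap only casts to Ball and takes no action.
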(event `self.ReceiveActorBeginOverlap`
  (params (OtherActor :type "Actor Object Reference"))
  (bind _asball (cast `/Game/Levels/BallThrow/Blueprints/Ball` OtherActor))
  (if (`PrimitiveComponent.IsOverlappingActor` (`self.Box`) _asball)
    (if (`PrimitiveComponent.IsOverlappingActor` (`self.Capsule`) _asball)
      (`KismetSystemLibrary.PrintString` "Hit" :!label _label)
      (`self.VerifyTry` true)
      (else
        (`KismetSystemLibrary.PrintString` "Fail")
        (`self.VerifyTry` false)))
    (else
      (goto _label))))

(event `self.ReceiveActorEndOverlap`
  (params (OtherActor :type "Actor Object Reference"))
  (cast `/Game/Levels/BallThrow/Blueprints/Ball` OtherActor))

(fn `UserConstructionScript`)