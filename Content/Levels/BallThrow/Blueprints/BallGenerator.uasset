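; BallGenerator is an actor in the BallThrow level that spawns a Ball at its Well component.
; While a FirstPersonCharacter overlaps it, GenerateBall is bound to that character's EventGenerateBall dispatcher, then unbound when the overlap ends.
; GenerateBall spawns a scaled-up Ball only if BallReady is set, then clears the flag until PrepareBall sets it again.
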(event `PrepareBall`
  (set `self.ballReady` true))

(event `self.ReceiveActorBeginOverlap`
  (params (OtherActor :type "Actor Object Reference"))
  (bind _asfirst_person_character (cast `/Game/FirstPersonCPP/Blueprints/FirstPersonCharacter` OtherActor))
  (add `/Game/FirstPersonCPP/Blueprints/FirstPersonCharacter.Event GenerateBall` _asfirst_person_character (delegate `GenerateBall`)))

(event `self.ReceiveActorEndOverlap`
  (params (OtherActor :type "Actor Object Reference"))
  (bind _asfirst_person_character (cast `/Game/FirstPersonCPP/Blueprints/FirstPersonCharacter` OtherActor))
  (remove `/Game/FirstPersonCPP/Blueprints/FirstPersonCharacter.Event GenerateBall` _asfirst_person_character (delegate `GenerateBall`)))

(event `GenerateBall`
  (if (`self.ballReady`)
    (`|SpawnActorFromClass` "/Game/Levels/BallThrow/Blueprints/Ball.Ball_C" (`KismetMathLibrary.ComposeTransforms` (`KismetMathLibrary.MakeTransform` (0.0 0.0 0.0) (struct) (5.0 5.0 4.0)) (`SceneComponent.K2_GetComponentToWorld` (`self.well`))) "Undefined" "OverrideRootScale")
    (set `self.ballReady` false)))

(fn `UserConstructionScript`)